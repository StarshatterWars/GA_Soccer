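; Football actor that stays with the possessing player and travels for passes, shots and misses by both teams.
; Each action event turns the ball toward its target and opens a Gate, letting Tick sweep it forward by PassSpeed each frame, unscaled by delta time.
; Overlapping the target closes the Gate and fires pass, goal or miss dispatchers.
; Completed passes also set the new possessor, which Tick follows at an offset for dribbling.
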(event Custom|EnemyShoot
  (params (Target :type Actor%20Object%20Reference))
  (bind _returnvalue (Transformation|GetActorLocation))
  (bind _returnvalue_2 (Transformation|GetActorForwardVector))
  (bind (_x _y) (Math|Vector|BreakVector _returnvalue_2))
  ;[1 1 1] Enemy Shooting
  (Transformation|SetActorRotation (Math|Rotator|FindLookatRotation _returnvalue (Transformation|GetActorLocation Target)))
  (Utilities|FlowControl|Gate true) ; enters at Open
)

(event Custom|EnemyMiss
  (params (Target :type Actor%20Object%20Reference))
  (bind _returnvalue (Transformation|GetActorLocation))
  (bind _returnvalue_2 (Transformation|GetActorForwardVector))
  (bind (_x _y) (Math|Vector|BreakVector _returnvalue_2))
  ;[1 1 1] Enemy Missing
  (Transformation|SetActorRotation (Math|Rotator|FindLookatRotation _returnvalue (Transformation|GetActorLocation Target)))
  (Utilities|FlowControl|Gate true) ; enters at Open
)

(event Custom|BallPassedMiss
  (params (ToMoveTo :type Actor%20Object%20Reference))
  (bind _returnvalue (Transformation|GetActorLocation))
  (bind _returnvalue_2 (Transformation|GetActorForwardVector))
  (bind (_x _y) (Math|Vector|BreakVector _returnvalue_2))
  ;[1 1 1] Passing to Enemy
  (Transformation|SetActorRotation (Math|Rotator|FindLookatRotation _returnvalue (Transformation|GetActorLocation ToMoveTo)))
  (Utilities|FlowControl|Gate true) ; enters at Open
)

(event Custom|Shooting
  (params (Goal :type Actor%20Object%20Reference))
  (bind _returnvalue (Transformation|GetActorLocation))
  (bind _returnvalue_2 (Transformation|GetActorForwardVector))
  (bind (_x _y) (Math|Vector|BreakVector _returnvalue_2))
  ;[1 1 1] Shooting
  (Transformation|SetActorRotation (Math|Rotator|FindLookatRotation _returnvalue (Transformation|GetActorLocation Goal)))
  (Utilities|FlowControl|Gate true) ; enters at Open
)

(event Custom|Missing
  (params (Target :type Actor%20Object%20Reference))
  (bind _returnvalue (Transformation|GetActorLocation))
  (bind _returnvalue_2 (Transformation|GetActorForwardVector))
  (bind (_x _y) (Math|Vector|BreakVector _returnvalue_2))
  ;[1 1 1] Missing
  (Transformation|SetActorRotation (Math|Rotator|FindLookatRotation _returnvalue (Transformation|GetActorLocation Target)))
  (Utilities|FlowControl|Gate true) ; enters at Open
)

(event Custom|BallPassed
  (params (ToMoveTo :type Actor%20Object%20Reference))
  (bind _returnvalue (Transformation|GetActorLocation))
  (bind _returnvalue_2 (Transformation|GetActorForwardVector))
  (bind (_x _y) (Math|Vector|BreakVector _returnvalue_2))
  ;[1 1 1] Passing to Friendly
  (Transformation|SetActorRotation (Math|Rotator|FindLookatRotation _returnvalue (Transformation|GetActorLocation ToMoveTo)))
  (Utilities|FlowControl|Gate true) ; enters at Open
)

(event EventTick
  (params (DeltaSeconds :type Float%20%28single-precision%29))
  (bind _returnvalue (Transformation|GetActorForwardVector))
  (bind _returnvalue_2 (Transformation|GetActorForwardVector))
  (bind _returnvalue_3 (Transformation|GetActorForwardVector))
  (bind _returnvalue_4 (Transformation|GetActorForwardVector))
  (bind _returnvalue_5 (Transformation|GetActorForwardVector))
  (bind _returnvalue_6 (Transformation|GetActorForwardVector))
  (bind _playerinpossession (Variables|Default|GetPlayerInPossession))
  (bind (_x _y) (Math|Vector|BreakVector _returnvalue))
  (bind (_x_2 _y_2) (Math|Vector|BreakVector _returnvalue_2))
  (bind (_x_3 _y_3) (Math|Vector|BreakVector _returnvalue_3))
  (bind (_x_4 _y_4) (Math|Vector|BreakVector _returnvalue_4))
  (bind (_x_5 _y_5) (Math|Vector|BreakVector _returnvalue_5))
  (bind (_x_6 _y_6) (Math|Vector|BreakVector _returnvalue_6))
  (Utilities|FlowControl|Sequence
    (:then_0
      ;[1 1 1] Dribbling
      (if (Variables|Default|GetBallPossessed)
        (Transformation|SetActorLocation (- (+ (* (Transformation|GetActorForwardVector _playerinpossession) (Variables|Default|GetBallDistanceOffset)) (Transformation|GetActorLocation _playerinpossession)) "0, 0,100.000000") false)))
    (:then_1
      ;[1 1 1] Passing to Friendly
      (Utilities|FlowControl|Gate true
        (:Exit
          (Transformation|SetActorRelativeLocation (+ (* (Math|Vector|MakeVector _x_6 _y_6 0.0) (Variables|Default|GetPassSpeed)) (Transformation|GetActorLocation)) true))))
    (:then_2
      ;[1 1 1] Shooting
      (Utilities|FlowControl|Gate true
        (:Exit
          (Transformation|SetActorRelativeLocation (+ (* (Math|Vector|MakeVector _x _y 0.0) (Variables|Default|GetPassSpeed)) (Transformation|GetActorLocation)) true))))
    (:then_3
      ;[1 1 1] Missing
      (Utilities|FlowControl|Gate true
        (:Exit
          (Transformation|SetActorRelativeLocation (+ (* (Math|Vector|MakeVector _x_2 _y_2 0.0) (Variables|Default|GetPassSpeed)) (Transformation|GetActorLocation)) true))))
    (:then_4
      ;[1 1 1] Passing to Enemy
      (Utilities|FlowControl|Gate true
        (:Exit
          (Transformation|SetActorRelativeLocation (+ (* (Math|Vector|MakeVector _x_3 _y_3 0.0) (Variables|Default|GetPassSpeed)) (Transformation|GetActorLocation)) true))))
    (:then_5
      ;[1 1 1] Enemy Shooting
      (Utilities|FlowControl|Gate true
        (:Exit
          (Transformation|SetActorRelativeLocation (+ (* (Math|Vector|MakeVector _x_5 _y_5 0.0) (Variables|Default|GetPassSpeed)) (Transformation|GetActorLocation)) true))))
    (:then_6
      ;[1 1 1] Enemy Missing
      (Utilities|FlowControl|Gate true
        (:Exit
          (Transformation|SetActorRelativeLocation (+ (* (Math|Vector|MakeVector _x_4 _y_4 0.0) (Variables|Default|GetPassSpeed)) (Transformation|GetActorLocation)) true))))))

(event EventBeginPlay
  (Variables|Default|SetStartLoc (Transformation|GetActorLocation)))

(event EventActorBeginOverlap
  (params (OtherActor :type Actor%20Object%20Reference))
  (bind _returnvalue (Transformation|GetActorForwardVector))
  (bind _returnvalue_2 (Transformation|GetActorForwardVector))
  (bind _returnvalue_3 (Transformation|GetActorForwardVector))
  (bind _returnvalue_4 (Transformation|GetActorForwardVector))
  (bind _returnvalue_5 (Transformation|GetActorForwardVector))
  (bind _returnvalue_6 (Transformation|GetActorForwardVector))
  (bind (_x _y) (Math|Vector|BreakVector _returnvalue))
  (bind (_x_2 _y_2) (Math|Vector|BreakVector _returnvalue_2))
  (bind (_x_3 _y_3) (Math|Vector|BreakVector _returnvalue_3))
  (bind (_x_4 _y_4) (Math|Vector|BreakVector _returnvalue_4))
  (bind (_x_5 _y_5) (Math|Vector|BreakVector _returnvalue_5))
  (bind (_x_6 _y_6) (Math|Vector|BreakVector _returnvalue_6))
  (Utilities|FlowControl|Sequence
    (:then_0
      ;[1 1 1] Passing to Friendly
      (if (== OtherActor (stale Custom|BallPassed ToMoveTo))
        (Utilities|FlowControl|Sequence
          (:then_0
            (Utilities|FlowControl|Gate true) ; enters at Close
          )
          (:then_1
            (Variables|Default|SetPlayerInPossession OtherActor)
            (Variables|Default|SetBallPossessed true)
            (Default|CallPassCompleted)))))
    (:then_1
      ;[1 1 1] Shooting
      (if (== OtherActor (stale Custom|Shooting Goal))
        (Utilities|FlowControl|Delay 0.2)
        (Default|CallGoalScored)
        (Utilities|FlowControl|Gate true) ; enters at Close
      ))
    (:then_2
      ;[1 1 1] Missing
      (if (== OtherActor (stale Custom|Missing Target))
        (Utilities|FlowControl|Delay 0.2)
        (Default|CallGoalMissed)
        (Utilities|FlowControl|Gate true) ; enters at Close
      ))
    (:then_3
      ;[1 1 1] Passing to Enemy
      (if (== OtherActor (stale Custom|BallPassedMiss ToMoveTo))
        (Utilities|FlowControl|Sequence
          (:then_0
            (Utilities|FlowControl|Gate true) ; enters at Close
          )
          (:then_1
            (Variables|Default|SetPlayerInPossession OtherActor)
            (Variables|Default|SetBallPossessed true)
            (Default|CallBadPassCompleted)))))
    (:then_4
      ;[1 1 1] Enemy Shooting
      (if (== OtherActor (stale Custom|EnemyShoot Target))
        (Utilities|FlowControl|Delay 0.2)
        (Default|CallEnemyGoalScored)
        (Utilities|FlowControl|Gate true) ; enters at Close
      ))
    (:then_5
      ;[1 1 1] Enemy Missing
      (if (== OtherActor (stale Custom|EnemyMiss Target))
        (Utilities|FlowControl|Delay 0.2)
        (Default|CallEnemyGoalMissed)
        (Utilities|FlowControl|Gate true) ; enters at Close
      ))))

(fn ConstructionScript)