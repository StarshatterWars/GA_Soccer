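; MyHUD is a HUD Blueprint that shows the friendly and enemy scores at the top of the screen during play.
; On each DrawHUD event it reads the screen size and draws both score variables as large white text on either side of the horizontal center.
; Nothing in this file updates the scores; it only renders their current values.
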(event EventDrawHUD
  (params (SizeX :type Integer) (SizeY :type Integer))
  (Variables|Default|SetScreenDimensions (Math|Vector2D|MakeVector2D (Math|Conversions|ToFloat(Integer) SizeX) (Math|Conversions|ToFloat(Integer) SizeY)))
  (HUD|DrawText (Utilities|String|ToString(Integer) (Variables|Default|GetFriendlyScore)) "(R=1.000000,G=1.000000,B=1.000000,A=1.000000)" (- (/ (.X (Math|Vector2D|BreakVector2D (Variables|Default|GetScreenDimensions))) 2.0) 65.0) 1e+01 "/Engine/EngineFonts/RobotoDistanceField.RobotoDistanceField" 3.0 false)
  (HUD|DrawText (Utilities|String|ToString(Integer) (Variables|Default|GetEnemyScore)) "(R=1.000000,G=1.000000,B=1.000000,A=1.000000)" (+ (/ (.X (Math|Vector2D|BreakVector2D (Variables|Default|GetScreenDimensions))) 2.0) 35.0) 1e+01 "/Engine/EngineFonts/RobotoDistanceField.RobotoDistanceField" 3.0 false))

(fn ConstructionScript)